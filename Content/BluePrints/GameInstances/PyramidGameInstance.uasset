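; Game instance that handles Epic Online Services sign-in and a WebSocket link to a local JVM process.
; On Init it tries persistent EOS auth, then falls back to a second login with default credentials, printing the outcome.
; Separate functions show the login widget, bind a login-ready event, and open the socket, checking the connection immediately after connecting.
; A message handler decodes JSON from the JVM and broadcasts it through MessageRecievedFromJava.
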(event `self.ReceiveInit`
  (bind _data (`EOSCoreAuthLogin.EOSAuthLoginAsync` (make `EOSAuthLoginOptions` (make `EOSAuthCredentials` "" "" "EOS_LCT_PersistentAuth")))
    (:`OnCallback`
      (if (`|EnumEquality` (`.ResultCode` (break `EOSAuthLoginCallbackInfo` _data)) "EOS_Success")
        (`KismetSystemLibrary.PrintString` "Welcome Back!")
        (else
          (bind _data_2 (`EOSCoreAuthLogin.EOSAuthLoginAsync` (make `EOSAuthLoginOptions` (make `EOSAuthCredentials` "")))
            (:`OnCallback`
              (if (`|EnumEquality` (`.ResultCode` (break `EOSAuthLoginCallbackInfo` _data_2)) "EOS_Success")
                (`KismetSystemLibrary.PrintString` "Account created successfully")
                (else
                  (`KismetSystemLibrary.PrintString` "Could not connect to EOS"))))))))))

(fn `Connect to JVM`
  (bind _output_get (set `self.JVMConnection` (`BlueprintWebSocket.CreateWebSocket`)))
  (`BlueprintWebSocket.Connect` _output_get "ws://localhost:9090" "ws")
  (if (`BlueprintWebSocket.IsConnected` _output_get)
    (`KismetSystemLibrary.PrintString` "Connection Successful!" true true (struct :`G` 0.66 :`B` 1.0 :`A` 1.0) 5.0)
    (add `BlueprintWebSocket.OnMessageEvent` _output_get (`|CreateDelegate` :!event `Handle Message From JVM`))
    (else
      (`KismetSystemLibrary.PrintString` "CONNECTION FAILURE!!" true true (struct :`R` 1.0 :`G` 0.021831 :`B` 0.151561 :`A` 1.0) 5.0))))

(fn `Handle Message From JVM`
  (params (MessageString :type String))
  (bind _output_get (set `self.json` (`|MakeJson`)))
  (bind _returnvalue (`VaRestJsonObject.DecodeJson` _output_get MessageString true))
  (if _returnvalue
    (`self.Message Recieved From Java` _output_get)
    (else
      (`KismetSystemLibrary.PrintString` "INVALID JSON RECIEVED" true true (struct :`G` 0.66 :`B` 1.0 :`A` 1.0) 5.0))))

(fn `Login`
  (bind _returnvalue (`|CreateWidget` "/Game/BluePrints/Widgets/WBP_Login.WBP_Login_C"))
  (`UserWidget.AddToViewport` _returnvalue 0))

(fn `LoginWhenReady`
  (add `self.LoginReady` (`|CreateDelegate` :!event `Login`)))