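; Character Blueprint for a modular mummy from the MummyPack, built from a body mesh plus separate armor, shield and weapon skeletal mesh pieces.
; On BeginPlay it sets every piece's master pose component to the main skeletal mesh, so all parts follow that mesh's animation.
; The construction script is empty and no other gameplay logic is present.
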(event `self.ReceiveBeginPlay`
  (`SkinnedMeshComponent.SetLeaderPoseComponent` (`self.Calf_Armor_L`) (`self.SkeletalMeshComponent`) false)
  (`SkinnedMeshComponent.SetLeaderPoseComponent` (`self.Calf_Armor_R`) (`self.SkeletalMeshComponent`) false)
  (`SkinnedMeshComponent.SetLeaderPoseComponent` (`self.Chest_Armor`) (`self.SkeletalMeshComponent`) false)
  (`SkinnedMeshComponent.SetLeaderPoseComponent` (`self.Forearm_Armor_L`) (`self.SkeletalMeshComponent`) false)
  (`SkinnedMeshComponent.SetLeaderPoseComponent` (`self.Head_Armor`) (`self.SkeletalMeshComponent`) false)
  (`SkinnedMeshComponent.SetLeaderPoseComponent` (`self.Forearm_Armor_R`) (`self.SkeletalMeshComponent`) false)
  (`SkinnedMeshComponent.SetLeaderPoseComponent` (`self.Shield`) (`self.SkeletalMeshComponent`) false)
  (`SkinnedMeshComponent.SetLeaderPoseComponent` (`self.Shoulder_Armor_L`) (`self.SkeletalMeshComponent`) false)
  (`SkinnedMeshComponent.SetLeaderPoseComponent` (`self.Shoulder_Armor_R`) (`self.SkeletalMeshComponent`) false)
  (`SkinnedMeshComponent.SetLeaderPoseComponent` (`self.UpperArm_Armor_L`) (`self.SkeletalMeshComponent`) false)
  (`SkinnedMeshComponent.SetLeaderPoseComponent` (`self.UpperArm_Armor_R`) (`self.SkeletalMeshComponent`) false)
  (`SkinnedMeshComponent.SetLeaderPoseComponent` (`self.Waist_Armor_A`) (`self.SkeletalMeshComponent`) false)
  (`SkinnedMeshComponent.SetLeaderPoseComponent` (`self.Waist_Armor_B`) (`self.SkeletalMeshComponent`) false)
  (`SkinnedMeshComponent.SetLeaderPoseComponent` (`self.Weapon`) (`self.SkeletalMeshComponent`) false))

(fn `UserConstructionScript`)